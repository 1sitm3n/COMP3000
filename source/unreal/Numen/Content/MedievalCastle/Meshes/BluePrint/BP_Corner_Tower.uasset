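; Procedural castle corner tower that assembles itself from static mesh components in the Construction Script, with no runtime logic.
; OpenWays selects the mesh variant for the base and each level above it.
; FloorNumbers (3 to 8) stacks alternating M1 and M2 middle levels at 360-unit steps under an MT level, with three floors having only MT above the base.
; LiftTopPart_2 then adds the top piece at a height computed from FloorNumbers.
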(event EventBeginPlay)

(event Collision|EventActorBeginOverlap
  (params (OtherActor :type Actor%20Object%20Reference)))

(event EventTick
  (params (DeltaSeconds :type Float%20%28single-precision%29)))

(fn ConstructionScript
  (bind _returnvalue (Math|Conversions|ToTransform(Vector) "0, 0,2160.000000"))
  (bind _returnvalue_2 (Math|Conversions|ToTransform(Vector) "0, 0,1800.000000"))
  (bind _returnvalue_3 (Math|Conversions|ToTransform(Vector) "0, 0,720.000000"))
  (bind _returnvalue_4 (Math|Conversions|ToTransform(Vector) "0,0.000000,1080.000000"))
  (bind _returnvalue_5 (Math|Conversions|ToTransform(Vector) "0, 0,360.000000"))
  (bind _returnvalue_6 (Math|Conversions|ToTransform(Vector) "0, 0,1440.000000"))
  ;[1 1 1] Base Level
  (|MainTower3ways
    (:1%20way
      _)
    (:2%20way
      _)
    (:3%20way
      _)
    (:Default
      _))
  (switch int (Variables|Default|GetFloor%20Numbers)
    (:3
      ;[1 1 1] Build Main Tower
      (CallFunction|TowerLevelMT _returnvalue_5 _returnvalue_5 _returnvalue_5 _returnvalue_5))
    (:4
      (CallFunction|TowerLevelM1 _returnvalue_5 _returnvalue_5 _returnvalue_5 _returnvalue_5)
      (CallFunction|TowerLevelMT _returnvalue_3 _returnvalue_3 _returnvalue_3 _returnvalue_3))
    (:5
      (CallFunction|TowerLevelM1 _returnvalue_5 _returnvalue_5 _returnvalue_5 _returnvalue_5)
      (CallFunction|TowerLevelM2 _returnvalue_3 _returnvalue_3 _returnvalue_3 _returnvalue_3)
      (CallFunction|TowerLevelMT _returnvalue_4 _returnvalue_4 _returnvalue_4 _returnvalue_4))
    (:6
      (CallFunction|TowerLevelM1 _returnvalue_5 _returnvalue_5 _returnvalue_5 _returnvalue_5)
      (CallFunction|TowerLevelM2 _returnvalue_3 _returnvalue_3 _returnvalue_3 _returnvalue_3)
      (CallFunction|TowerLevelM1 _returnvalue_4 _returnvalue_4 _returnvalue_4 _returnvalue_4)
      (CallFunction|TowerLevelMT _returnvalue_6 _returnvalue_6 _returnvalue_6 _returnvalue_6))
    (:7
      (CallFunction|TowerLevelM1 _returnvalue_5 _returnvalue_5 _returnvalue_5 _returnvalue_5)
      (CallFunction|TowerLevelM2 _returnvalue_3 _returnvalue_3 _returnvalue_3 _returnvalue_3)
      (CallFunction|TowerLevelM1 _returnvalue_4 _returnvalue_4 _returnvalue_4 _returnvalue_4)
      (CallFunction|TowerLevelM2 _returnvalue_6 _returnvalue_6 _returnvalue_6 _returnvalue_6)
      (CallFunction|TowerLevelMT _returnvalue_2 _returnvalue_2 _returnvalue_2 _returnvalue_2))
    (:8
      (CallFunction|TowerLevelM1 _returnvalue_5 _returnvalue_5 _returnvalue_5 _returnvalue_5)
      (CallFunction|TowerLevelM2 _returnvalue_3 _returnvalue_3 _returnvalue_3 _returnvalue_3)
      (CallFunction|TowerLevelM1 _returnvalue_4 _returnvalue_4 _returnvalue_4 _returnvalue_4)
      (CallFunction|TowerLevelM2 _returnvalue_6 _returnvalue_6 _returnvalue_6 _returnvalue_6)
      (CallFunction|TowerLevelM1 _returnvalue_2 _returnvalue_2 _returnvalue_2 _returnvalue_2)
      (CallFunction|TowerLevelMT _returnvalue _returnvalue _returnvalue _returnvalue)))
  (|LiftTopPart_2))

(fn TowerLevelM2
  (params (RelativeTransform1 :type Transform) (RelativeTransform2 :type Transform) (RelativeTransform3 :type Transform) (RelativeTransform4 :type Transform))
  (switch int (Variables|Default|GetOpen%20Ways)
    (:0
      (AddComponent|AddStaticMeshComponent false RelativeTransform1))
    (:1
      (AddComponent|AddStaticMeshComponent false RelativeTransform2))
    (:2
      (AddComponent|AddStaticMeshComponent false RelativeTransform3))
    (:3
      (AddComponent|AddStaticMeshComponent false RelativeTransform4))))

(fn TowerLevelM1
  (params (RelativeTransform1 :type Transform) (RelativeTransform2 :type Transform) (RelativeTransform3 :type Transform) (RelativeTransform4 :type Transform))
  (switch int (Variables|Default|GetOpen%20Ways)
    (:0
      (AddComponent|AddStaticMeshComponent false RelativeTransform1))
    (:1
      (AddComponent|AddStaticMeshComponent false RelativeTransform2))
    (:2
      (AddComponent|AddStaticMeshComponent false RelativeTransform3))
    (:3
      (AddComponent|AddStaticMeshComponent false RelativeTransform4))))

(fn TowerLevelMT
  (params (RelativeTransform :type Transform) (RelativeTransform2 :type Transform) (RelativeTransform3 :type Transform) (RelativeTransform4 :type Transform))
  (switch int (Variables|Default|GetOpen%20Ways)
    (:0
      (AddComponent|AddStaticMeshComponent false RelativeTransform))
    (:1
      (AddComponent|AddStaticMeshComponent false RelativeTransform2))
    (:2
      (AddComponent|AddStaticMeshComponent false RelativeTransform3))
    (:3
      (AddComponent|AddStaticMeshComponent false RelativeTransform4))))