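; Procedural castle corridor actor that builds a multi-storey corridor from modular static meshes in its Construction Script.
; A switch on FloorNumber (one to six) stacks a base level, alternating M1 and M2 middle levels, and a top level.
; Each level function repeats its mesh along X Length times at a fixed spacing.
; The top level's height is computed from FloorNumber, while lower levels use fixed offsets.
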(event EventBeginPlay)

(event Collision|EventActorBeginOverlap
  (params (OtherActor :type Actor%20Object%20Reference)))

(event EventTick
  (params (DeltaSeconds :type Float%20%28single-precision%29)))

(fn ConstructionScript
  (bind _returnvalue (Math|Conversions|ToTransform(Vector) "0, 0,360.000000"))
  (bind _returnvalue_2 (Math|Conversions|ToTransform(Vector) "0, 0,1080.000000"))
  (bind _returnvalue_3 (Math|Conversions|ToTransform(Vector) "0, 0,1440.000000"))
  (bind _returnvalue_4 (Math|Conversions|ToTransform(Vector) "0, 0, 0"))
  (bind _returnvalue_5 (Math|Conversions|ToTransform(Vector) "0, 0,720.000000"))
  (bind _floor_number (Variables|Default|GetFloor%20Number))
  (switch int _floor_number
    (:1
      (CallFunction|CorridorUnitLevelBase _returnvalue_4))
    (:2
      (CallFunction|CorridorUnitLevelBase _returnvalue_4)
      (CallFunction|CorridorUnitLevleM1 _returnvalue))
    (:3
      (CallFunction|CorridorUnitLevelBase _returnvalue_4)
      (CallFunction|CorridorUnitLevleM1 _returnvalue)
      (CallFunction|CorridorUnitLevelM2 _returnvalue_5))
    (:4
      (CallFunction|CorridorUnitLevelBase _returnvalue_4)
      (CallFunction|CorridorUnitLevleM1 _returnvalue)
      (CallFunction|CorridorUnitLevelM2 _returnvalue_5)
      (CallFunction|CorridorUnitLevleM1 _returnvalue_2))
    (:5
      (CallFunction|CorridorUnitLevelBase _returnvalue_4)
      (CallFunction|CorridorUnitLevleM1 _returnvalue)
      (CallFunction|CorridorUnitLevelM2 _returnvalue_5)
      (CallFunction|CorridorUnitLevleM1 _returnvalue_2)
      (CallFunction|CorridorUnitLevelM2 _returnvalue_3))
    (:6
      (CallFunction|CorridorUnitLevelBase _returnvalue_4)
      (CallFunction|CorridorUnitLevleM1 _returnvalue)
      (CallFunction|CorridorUnitLevelM2 _returnvalue_5)
      (CallFunction|CorridorUnitLevleM1 _returnvalue_2)
      (CallFunction|CorridorUnitLevelM2 _returnvalue_3)
      (CallFunction|CorridorUnitLevleM1 (Math|Conversions|ToTransform(Vector) "0, 0,1800.000000"))))
  (CallFunction|CorridorUnitLevelTop (Math|Conversions|ToTransform(Vector) (Math|Vector|MakeVector 0.0 0.0 (Math|Conversions|ToFloat(Integer) (+ 340 (* (- _floor_number 1) 360)))))))

(fn CorridorUnitLevelBase
  (params (RelativeTransform :type Transform))
  (for _index (range 0 (- (Variables|Default|GetLength) 1))
    (AddComponent|AddStaticMeshComponent false (Math|Conversions|ToTransform(Vector) (+ (Math|Vector|MakeVector (Math|Conversions|ToFloat(Integer) (* _index 665)) 0.0 0.0) (.Location (Math|Transform|BreakTransform RelativeTransform)))))))

(fn CorridorUnitLevleM1
  (params (RelativeTransform :type Transform))
  (for _index (range 0 (- (Variables|Default|GetLength) 1))
    (AddComponent|AddStaticMeshComponent false (Math|Conversions|ToTransform(Vector) (+ (Math|Vector|MakeVector (Math|Conversions|ToFloat(Integer) (* _index 665)) 0.0 0.0) (.Location (Math|Transform|BreakTransform RelativeTransform)))))))

(fn CorridorUnitLevelM2
  (params (RelativeTransform :type Transform))
  (for _index (range 0 (- (Variables|Default|GetLength) 1))
    (AddComponent|AddStaticMeshComponent false (Math|Conversions|ToTransform(Vector) (+ (Math|Vector|MakeVector (Math|Conversions|ToFloat(Integer) (* _index 665)) 0.0 0.0) (.Location (Math|Transform|BreakTransform RelativeTransform)))))))

(fn CorridorUnitLevelTop
  (params (InTransform :type Transform%20%28by%20ref%29))
  (for _index (range 0 (- (Variables|Default|GetLength) 1))
    (AddComponent|AddStaticMeshComponent false (Math|Conversions|ToTransform(Vector) (+ (Math|Vector|MakeVector (Math|Conversions|ToFloat(Integer) (* _index 665)) 0.0 0.0) (.Location (Math|Transform|BreakTransform InTransform)))))))