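; BP_FrontHall is a construction-script building piece that procedurally stacks a castle front hall from static mesh components according to FloorNumber.
; It places fixed lower pieces, then loops to add middle floors at even vertical spacing.
; Two top-floor pieces are positioned from FloorNumber; that branch runs both inside the loop and on completion, so it adds overlapping duplicates when middle floors exist.
; The event graph is unused.
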(event EventBeginPlay)

(event Collision|EventActorBeginOverlap
  (params (OtherActor :type Actor%20Object%20Reference)))

(event EventTick
  (params (DeltaSeconds :type Float%20%28single-precision%29)))

(fn ConstructionScript
  (bind _floor_number (Variables|Default|GetFloor%20Number))
  (bind _returnvalue (- _floor_number 1))
  (bind _returnvalue_2 (* _returnvalue 360))
  (AddComponent|AddStaticMeshComponent false)
  (AddComponent|AddStaticMeshComponent false (Math|Conversions|ToTransform(Vector) "0, 0,720.000000"))
  ;[1 1 1] Middle Floors
  (for _index (range 4 _returnvalue)
    (AddComponent|AddStaticMeshComponent false (Math|Conversions|ToTransform(Vector) (Math|Vector|MakeVector 0.0 0.0 (Math|Conversions|ToFloat(Integer) (+ (* (- _index 4) 360) 1080)))))
    ;[1 1 1] Top Floor
    (AddComponent|AddStaticMeshComponent false (Math|Conversions|ToTransform(Vector) (Math|Vector|MakeVector 0.0 0.0 (Math|Conversions|ToFloat(Integer) _returnvalue_2))))
    (AddComponent|AddStaticMeshComponent false (Math|Conversions|ToTransform(Vector) (Math|Vector|MakeVector 0.0 0.0 (Math|Conversions|ToFloat(Integer) (+ _returnvalue_2 360))))))
  (AddComponent|AddStaticMeshComponent false (Math|Conversions|ToTransform(Vector) (Math|Vector|MakeVector 0.0 0.0 (Math|Conversions|ToFloat(Integer) _returnvalue_2))))
  (AddComponent|AddStaticMeshComponent false (Math|Conversions|ToTransform(Vector) (Math|Vector|MakeVector 0.0 0.0 (Math|Conversions|ToFloat(Integer) (+ _returnvalue_2 360))))))