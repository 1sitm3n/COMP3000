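; BP_MainHall is a procedural castle main hall building whose height is driven by FloorNumber.
; The construction script adds one static mesh at the origin and another offset vertically to FloorNumber minus two floors.
; A loop stacks intermediate meshes at 360-unit intervals between them, starting at the second floor offset.
; The event graph holds only disabled stub events, so there is no runtime logic.
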(event EventBeginPlay)

(event Collision|EventActorBeginOverlap
  (params (OtherActor :type Actor%20Object%20Reference)))

(event EventTick
  (params (DeltaSeconds :type Float%20%28single-precision%29)))

(fn ConstructionScript
  (AddComponent|AddStaticMeshComponent false)
  (AddComponent|AddStaticMeshComponent false (Math|Conversions|ToTransform(Vector) (Math|Vector|MakeVector 0.0 0.0 (Math|Conversions|ToFloat(Integer) (* (- (Variables|Default|GetFloor%20Number) 2) 360)))))
  (for _index (range 2 (- (Variables|Default|GetFloor%20Number) 3))
    (AddComponent|AddStaticMeshComponent false (Math|Conversions|ToTransform(Vector) (Math|Vector|MakeVector 0.0 0.0 (Math|Conversions|ToFloat(Integer) (* (- _index 0) 360)))))))