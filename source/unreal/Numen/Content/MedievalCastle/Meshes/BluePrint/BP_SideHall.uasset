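; Procedural medieval castle side hall that assembles a stackable building from static meshes, sized by FloorNumber.
; The Construction Script places a base mesh, then loops over floors at 360-unit spacing, adding storey and top pieces.
; Inside that loop, a switch on FloorNumber (3 to 8) stacks exterior walls through per-level helper functions, reusing the I5 wall for the highest level.
; Event graph is inactive, and child-actor helper NewFunction_3 is never called.
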(event EventBeginPlay)

(event Collision|EventActorBeginOverlap
  (params (OtherActor :type Actor%20Object%20Reference)))

(event EventTick
  (params (DeltaSeconds :type Float%20%28single-precision%29)))

(fn ConstructionScript
  (bind _returnvalue (Math|Conversions|ToTransform(Vector) "0, 0,1800.000000"))
  (bind _returnvalue_2 (Math|Conversions|ToTransform(Vector) "0, 0,360.000000"))
  (bind _returnvalue_3 (Math|Conversions|ToTransform(Vector) "0, 0,720.000000"))
  (bind _returnvalue_4 (Math|Conversions|ToTransform(Vector) "0, 0,1080.000000"))
  (bind _returnvalue_5 (Math|Conversions|ToTransform(Vector) "0, 0,1440.000000"))
  (bind _floor_number (Variables|Default|GetFloor%20Number))
  (AddComponent|AddStaticMeshComponent false)
  (for _index (range 3 (- _floor_number 0))
    (AddComponent|AddStaticMeshComponent false (Math|Conversions|ToTransform(Vector) (Math|Vector|MakeVector 0.0 0.0 (Math|Conversions|ToFloat(Integer) (* (- _index 2) 360)))))
    (AddComponent|AddStaticMeshComponent false (Math|Conversions|ToTransform(Vector) (Math|Vector|MakeVector 0.0 0.0 (Math|Conversions|ToFloat(Integer) (+ (* (- _floor_number 2) 360) 360)))))
    ;[1 1 1] Exterior Wall Combination
    (switch int (Variables|Default|GetFloor%20Number)
      (:3
        (CallFunction|WallEXMI2 _returnvalue_2))
      (:4
        (CallFunction|WallEXMI2 _returnvalue_2)
        (CallFunction|WallEXMI3 _returnvalue_3))
      (:5
        (CallFunction|WallEXMI2 _returnvalue_2)
        (CallFunction|WallEXMI3 _returnvalue_3)
        (CallFunction|WallEXMI4 _returnvalue_4))
      (:6
        (CallFunction|WallEXMI2 _returnvalue_2)
        (CallFunction|WallEXMI3 _returnvalue_3)
        (CallFunction|WallEXMI4 _returnvalue_4)
        (CallFunction|WallEXMI5 _returnvalue_5))
      (:7
        (CallFunction|WallEXMI2 _returnvalue_2)
        (CallFunction|WallEXMI3 _returnvalue_3)
        (CallFunction|WallEXMI4 _returnvalue_4)
        (CallFunction|WallEXMI5 _returnvalue_5)
        (CallFunction|WallEXMI6 _returnvalue))
      (:8
        (CallFunction|WallEXMI2 _returnvalue_2)
        (CallFunction|WallEXMI3 _returnvalue_3)
        (CallFunction|WallEXMI4 _returnvalue_4)
        (CallFunction|WallEXMI5 _returnvalue_5)
        (CallFunction|WallEXMI6 _returnvalue)
        (CallFunction|WallEXMI5 (Math|Conversions|ToTransform(Vector) "0, 0,2160.000000"))))))

(fn WallEXMI2
  (params (RelativeTransform :type Transform))
  (AddComponent|AddStaticMeshComponent false RelativeTransform))

(fn WallEXMI3
  (params (RelativeTransform :type Transform))
  (AddComponent|AddStaticMeshComponent false RelativeTransform))

(fn WallEXMI4
  (params (RelativeTransform :type Transform))
  (AddComponent|AddStaticMeshComponent false RelativeTransform))

(fn WallEXMI5
  (params (RelativeTransform :type Transform))
  (AddComponent|AddStaticMeshComponent false RelativeTransform))

(fn NewFunction3
  (params (RelativeTransform :type Transform))
  (AddComponent|AddChildActorComponent false RelativeTransform))

(fn WallEXMI6
  (params (RelativeTransform :type Transform))
  (AddComponent|AddStaticMeshComponent false RelativeTransform))