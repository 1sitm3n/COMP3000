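; Actor component that assembles a modular elf character by swapping skeletal meshes on its owner.
; SetupCharacter first finds mesh components tagged Hair, Head, Body, Hands and Outfit, printing errors for missing tags and warnings for duplicates.
; It then assigns meshes by index, with hair index zero using a head-matched variant and hands optionally emptied.
; The Outfit component is required, but OutfitIndex is unused and its mesh stays untouched.
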(fn ResolveSKMComponent
  (params (Tag :type Name))
  (bind _returnvalue (Utilities|String|ToString(Name) Tag))
  (LocalVariables|SetSKM%20Components (Actor|GetComponentsbyTag (Components|GetOwner) "/Script/Engine.SkeletalMeshComponent" Tag))
  (if (Utilities|Array|IsEmpty (LocalVariables|GetSKM%20Components))
    (Development|PrintString (Utilities|String|Append "Error: " _returnvalue " Component is Missing! Add an Skeletal Mesh With '" _returnvalue "' Tag.") true true "(R=1.000000,G=0.000000,B=0.000000,A=1.000000)" 1e+01)
    (return 0)
    (else
      (if (> (Utilities|Array|Length (LocalVariables|GetSKM%20Components)) 1)
        (Development|PrintString (Utilities|String|Append "Warning: Multiple Skeletal Mesh Components with '" (Utilities|String|ToString(Name) Tag) "' Tag found! Picking the first one.") true true "(R=1.000000,G=0.549683,B=0.000000,A=1.000000)" 1e+01))
      (return (Utilities|Array|Get(acopy) (LocalVariables|GetSKM%20Components))))))

(fn ResolveBodyparts
  (Utilities|FlowControl|Sequence
    (:then_0
      (bind _output (Utility|ResolveSKMComponent "Hair"))
      (bind _output_get (Variables|Default|SetHair _output))
      (Utilities|IsValid _output_get
        (:Is%20Not%20Valid
          (return false))))
    (:then_1
      (bind _output_2 (Utility|ResolveSKMComponent "Head"))
      (bind _output_get_2 (Variables|Default|SetHead _output_2))
      (Utilities|IsValid _output_get_2
        (:Is%20Not%20Valid
          (return false))))
    (:then_2
      (bind _output_3 (Utility|ResolveSKMComponent "Body"))
      (bind _output_get_3 (Variables|Default|SetBody _output_3))
      (Utilities|IsValid _output_get_3
        (:Is%20Not%20Valid
          (return false))))
    (:then_3
      (bind _output_4 (Utility|ResolveSKMComponent "Hands"))
      (bind _output_get_4 (Variables|Default|SetHands _output_4))
      (Utilities|IsValid _output_get_4
        (:Is%20Not%20Valid
          (return false))))
    (:then_4
      (bind _output_5 (Utility|ResolveSKMComponent "Outfit"))
      (bind _output_get_5 (Variables|Default|SetSingle%20Mesh%20Clothes _output_5))
      (Utilities|IsValid _output_get_5
        (:Is%20Not%20Valid
          (return false))))
    (:then_5
      (return true))))

(fn SetupCharacter
  (params (Hair%20Index :type Integer) (Head%20/%20Body%20Index :type Integer) (Outfit%20Index :type Integer) (Hide%20Hands :type Boolean))
  (Utilities|FlowControl|Sequence
    (:then_0
      ;[1 1 1] Resolve requered components
      (bind _success (Utility|ResolveBodyparts))
      (if (not _success)
        (Development|PrintString "Error: Could not resolve all the requered components!" true true "(R=1.000000,G=0.000000,B=0.000000,A=1.000000)" 1e+01)
        (return)))
    (:then_1
      ;[1 1 1] Hair Selection
      (Math|Integer|CompareInt Hair%20Index
        (:>
          (Components|SkeletalMesh|SetSkeletalMeshAsset (Variables|Default|GetHair) (Utilities|Array|Get(acopy) (Variables|Meshes|GetHair%20Meshes) Hair%20Index)))
        (:==
          (Components|SkeletalMesh|SetSkeletalMeshAsset (Variables|Default|GetHair) (Utilities|Array|Get(acopy) (Variables|Meshes|GetHair%20A%20Variations) Head%20/%20Body%20Index)))))
    (:then_2
      ;[1 1 1] Body Selection
      (Utilities|FlowControl|Sequence
        (:then_0
          (Components|SkeletalMesh|SetSkeletalMeshAsset (Variables|Default|GetHead) (Utilities|Array|Get(acopy) (Variables|Meshes|GetHead%20Meshes) Head%20/%20Body%20Index)))
        (:then_1
          (Components|SkeletalMesh|SetSkeletalMeshAsset (Variables|Default|GetBody) (Utilities|Array|Get(acopy) (Variables|Meshes|GetBody%20Meshes) Head%20/%20Body%20Index)))
        (:then_2
          (if Hide%20Hands
            (Components|SkeletalMesh|SetSkeletalMeshAsset (Variables|Default|GetHands) (Variables|Meshes|GetEmpty%20Mesh))
            (else
              (Components|SkeletalMesh|SetSkeletalMeshAsset (Variables|Default|GetHands) (Utilities|Array|Get(acopy) (Variables|Meshes|GetHand%20Meshes) Head%20/%20Body%20Index)))))))))